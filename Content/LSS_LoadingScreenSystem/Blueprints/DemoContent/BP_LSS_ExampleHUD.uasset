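; Example HUD for the Loading Screen System demo that hands out references to the demo's UI widgets.
; Getters cover the main menu, two game HUD variants, a tips loading screen and a complex press-space-to-continue screen.
; Each uses the shared Get UI Ref macro, which lazily creates the widget for player 0 and caches it by reference.
; It only creates widgets and does not add them to the viewport.
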(fn `Get UI Game HUD`
  (returns (`UI Ref` :type "UserWidget Object Reference"))
  (bind _ui_game_hud_ref (`self.UI Game HUD Ref`))
  (`self.Get UI Ref` "/Game/LSS_LoadingScreenSystem/UI/ExampleWidgets/UI_LSS_ExampleGameHud_A.UI_LSS_ExampleGameHud_A_C" _ui_game_hud_ref
    (:`Is Valid`
      (return _ui_game_hud_ref))))

(fn `Get UI Game HUD B`
  (returns (`UI Ref` :type "UserWidget Object Reference"))
  (bind _ui_game_hud_b_ref (`self.UI Game HUD B Ref`))
  (`self.Get UI Ref` "/Game/LSS_LoadingScreenSystem/UI/ExampleWidgets/UI_LSS_ExampleGameHud_B.UI_LSS_ExampleGameHud_B_C" _ui_game_hud_b_ref
    (:`Is Valid`
      (return _ui_game_hud_b_ref))))

(fn `Get UI Loading`
  (returns (`UI Ref` :type "UserWidget Object Reference"))
  (bind _ui_loading_ref (`self.UI Loading Ref`))
  (`self.Get UI Ref` "/Game/LSS_LoadingScreenSystem/UI/ExampleWidgets/UI_LSS_Tips.UI_LSS_Tips_C" _ui_loading_ref
    (:`Is Valid`
      (return _ui_loading_ref))))

(fn `Get UI Loading Complex`
  (returns (`UI Ref` :type "UserWidget Object Reference"))
  (bind _ui_loading_complex_ref (`self.UI Loading Complex Ref`))
  (`self.Get UI Ref` "/Game/LSS_LoadingScreenSystem/UI/ExampleWidgets/UI_LSS_PressSpaceToContinue_Complex.UI_LSS_PressSpaceToContinue_Complex_C" _ui_loading_complex_ref
    (:`Is Valid`
      (return _ui_loading_complex_ref))))

(fn `Get UI Main Menu`
  (returns (`UI Ref` :type "UserWidget Object Reference"))
  (bind _ui_main_menu_ref (`self.UI Main Menu Ref`))
  (`self.Get UI Ref` "/Game/LSS_LoadingScreenSystem/UI/ExampleWidgets/UI_LSS_ExampleMainMenu.UI_LSS_ExampleMainMenu_C" _ui_main_menu_ref
    (:`Is Valid`
      (return _ui_main_menu_ref))))

(fn `UserConstructionScript`)