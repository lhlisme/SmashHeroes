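; Demo room button that fires its ButtonToggled dispatcher when E is pressed while a pawn is in range.
; A trigger overlap and a delayed Tick range check switch the button's dynamic material state between red and green.
; The same check plays or reverses a timeline that scales the info text and raises the point light's intensity.
; Pressing E in range also resets the button to red.
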(event `Key|E` :consume false
  (params (Key :type "Key Structure"))
  (:`Pressed`
    (bind _returnvalue (`self.Is Pawn In Range`))
    (if _returnvalue
      (`|ExecutionSequence`
        (:`then_0`
          (`MaterialInstanceDynamic.SetScalarParameterValue` (`self.Button light material`) "State" 0.0 :!label _label) ; Change a scalar value in the button material that turns it back to red
        )
        (:`then_1`
          (`self.Button toggled` true))))))

(event `self.Trigger collision.OnComponentBeginOverlap`
  (params (OverlappedComponent :type "PrimitiveComponent Object Reference") (OtherActor :type "Actor Object Reference") (OtherComp :type "PrimitiveComponent Object Reference") (OtherBodyIndex :type Integer) (bFromSweep :type Boolean) (SweepResult :type "HitResult Structure (by ref)"))
  (`MaterialInstanceDynamic.SetScalarParameterValue` (`self.Button light material`) "State" 1.0 :!label _label_2) ; Change a scalar value in the button material that turns it green
)

(event `self.Trigger collision.OnComponentEndOverlap`
  (params (OverlappedComponent :type "PrimitiveComponent Object Reference") (OtherActor :type "Actor Object Reference") (OtherComp :type "PrimitiveComponent Object Reference") (OtherBodyIndex :type Integer))
  (goto _label))

(event `self.ReceiveTick`
  (params (DeltaSeconds :type "Float (single-precision)"))
  (`KismetSystemLibrary.Delay` 0.2)
  (bind _returnvalue (`self.Is Pawn In Range`))
  (if _returnvalue
    (`self.Show Info`)
    (goto _label_2)
    (else
      (`self.Hide Info`)
      (goto _label))))

(event `Show Info`
  (`TimelineComponent.SetPlayRate` (`self.Show Info Text`) 3.0)
  (bind (_direction _alpha) (`Timeline|Show Info Text` :!label _label_3)
    (:`Update`
      (`SceneComponent.SetRelativeScale3D` (`self.TextRender`) (`KismetMathLibrary.Conv_DoubleToVector` _alpha))
      (`LightComponent.SetIntensity` (`self.PointLight`) (`KismetMathLibrary.MapRangeClamped` _alpha 0.0 1.0 0.0 10000.0)))))

(event `Hide Info`
  (`TimelineComponent.SetPlayRate` (`self.Show Info Text`) 1.0)
  (goto _label_3 :!via `Reverse`))

(fn `Is Pawn In Range`
  (returns (ReturnValue :type Boolean))
  (bind _trigger_collision (`self.Trigger collision`))
  (bind (_outactors _returnvalue) (`KismetSystemLibrary.ComponentOverlapActors` _trigger_collision (`SceneComponent.K2_GetComponentToWorld` _trigger_collision) (`|MakeArray` "ObjectTypeQuery3" :!type "EObjectTypeQuery Enum")))
  (return _returnvalue))

(fn `UserConstructionScript`
  (bind _returnvalue (`PrimitiveComponent.CreateDynamicMaterialInstance` (`self.ButtonMesh`) 2 null))
  (set `self.Button light material` _returnvalue) ; Save a reference to the Dynamic Material Instance for use in the event graph
)