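; Projectile actor for the space shooter minigame in the loading screen system demo content, tinted by a color set at spawn.
; The construction script creates a dynamic material, which BeginPlay colors along with the light.
; Tick moves it along a local offset from its Speed variable without sweeping.
; On overlapping any actor except its owner, it applies fixed damage, spawns an explosion with impact sound, and destroys itself.
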(event `self.ReceiveBeginPlay`
  (bind _projectile_color (`self.Projectile color`))
  (bind _projectile_material (`self.Projectile material`))
  (`MaterialInstanceDynamic.SetVectorParameterValue` _projectile_material "Color2" _projectile_color) ; Set the projectile color
  (`MaterialInstanceDynamic.SetVectorParameterValue` _projectile_material "Color1" (* _projectile_color (struct :`R` 1.0 :`G` 0.5 :`B` 0.785131 :`A` 1.0))) ; Set the projectile color
  (`LightComponent.SetLightColor` (`self.Light`) _projectile_color true) ; Set the projectile's light color
)

(event `self.ReceiveTick`
  (params (DeltaSeconds :type "Float (single-precision)"))
  (`self.K2_AddActorLocalOffset` (* (`self.Speed`) DeltaSeconds)) ; Move projectile in the desired direction
)

(event `self.Projectile.OnComponentBeginOverlap`
  (params (OverlappedComponent :type "PrimitiveComponent Object Reference") (OtherActor :type "Actor Object Reference") (OtherComp :type "PrimitiveComponent Object Reference") (OtherBodyIndex :type Integer) (bFromSweep :type Boolean) (SweepResult :type "HitResult Structure (by ref)"))
  (bind _returnvalue (`self.K2_GetActorLocation`))
  (if (!= OtherActor (`self.Projectile owner`))
    (`GameplayStatics.ApplyDamage` OtherActor 20.0) ; Apply damage to the hit actor
    (`GameplayStatics.SpawnEmitterAtLocation` "/Game/LSS_LoadingScreenSystem/DemoContent/SpaceshooterMinigame/Effects/P_Pixel_Explosion.P_Pixel_Explosion" _returnvalue) ; Spawn an explosion emitter
    (`GameplayStatics.PlaySoundAtLocation` "/Game/LSS_LoadingScreenSystem/DemoContent/SpaceshooterMinigame/Audio/Cue/Arcade_Ship_FireImpact_Cue.Arcade_Ship_FireImpact_Cue" _returnvalue) ; Projectile impact sound
    (`self.K2_DestroyActor`) ; Destroy the projectile actor
  ))

(fn `UserConstructionScript`
  (bind _returnvalue (`PrimitiveComponent.CreateDynamicMaterialInstance` (`self.Projectile`) 0 null)) ; Create and apply a dynamic material instance for the projectile mesh
  (set `self.Projectile material` _returnvalue) ; Save as a variable so its properties can be changed in the event graph
)