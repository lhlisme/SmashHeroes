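; Right-hand paddle for the Pong minigame in the loading screen demo content, moving along the X axis.
; Each Tick moves it by MovementInput, Speed and delta time, or snaps it just inside the fixed X bounds when it overshoots.
; Top and bottom trigger boxes set MovementInput from Pawn overlaps for automatic steering.
; When it is player 0's pawn, forward-axis input overrides that value.
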(event `self.ReceiveTick`
  (params (DeltaSeconds :type "Float (single-precision)"))
  (if (> (.x (`self.K2_GetActorLocation`)) 1500.0)
    (`self.K2_SetActorLocation` (`KismetMathLibrary.MakeVector` 1499.0 (.y (`self.K2_GetActorLocation`)) (.z (`self.K2_GetActorLocation`))))
    (elif (< (.x (`self.K2_GetActorLocation`)) -1500.0)
      (`self.K2_SetActorLocation` (`KismetMathLibrary.MakeVector` -1499.0 (.y (`self.K2_GetActorLocation`)) (.z (`self.K2_GetActorLocation`))))
      (else
        (`|ExecutionSequence`
          (:`then_0`
            (if (== (`GameplayStatics.GetPlayerPawn` 0) self)
              (set `self.Movement Input` (`self.GetInputAxisValue`))))
          (:`then_1`
            (`self.K2_SetActorLocation` (`KismetMathLibrary.MakeVector` (+ (* (`self.Movement Input`) (* (`GameplayStatics.GetWorldDeltaSeconds`) (`self.Speed`))) (.x (`self.K2_GetActorLocation`))) (.y (`self.K2_GetActorLocation`)) (.z (`self.K2_GetActorLocation`))))))))))

(event `self.BoxBottom.OnComponentBeginOverlap`
  (params (OverlappedComponent :type "PrimitiveComponent Object Reference") (OtherActor :type "Actor Object Reference") (OtherComp :type "PrimitiveComponent Object Reference") (OtherBodyIndex :type Integer) (bFromSweep :type Boolean) (SweepResult :type "HitResult Structure (by ref)"))
  (cast `Pawn` OtherActor)
  (set `self.Movement Input` -1.0))

(event `self.BoxTop.OnComponentBeginOverlap`
  (params (OverlappedComponent :type "PrimitiveComponent Object Reference") (OtherActor :type "Actor Object Reference") (OtherComp :type "PrimitiveComponent Object Reference") (OtherBodyIndex :type Integer) (bFromSweep :type Boolean) (SweepResult :type "HitResult Structure (by ref)"))
  (cast `Pawn` OtherActor)
  (set `self.Movement Input` 1.0))

(event `self.BoxBottom.OnComponentEndOverlap`
  (params (OverlappedComponent :type "PrimitiveComponent Object Reference") (OtherActor :type "Actor Object Reference") (OtherComp :type "PrimitiveComponent Object Reference") (OtherBodyIndex :type Integer))
  (cast `Pawn` OtherActor)
  (set `self.Movement Input` 0.0))

(event `self.BoxTop.OnComponentEndOverlap`
  (params (OverlappedComponent :type "PrimitiveComponent Object Reference") (OtherActor :type "Actor Object Reference") (OtherComp :type "PrimitiveComponent Object Reference") (OtherBodyIndex :type Integer))
  (cast `Pawn` OtherActor)
  (set `self.Movement Input` 0.0))

(fn `UserConstructionScript`)