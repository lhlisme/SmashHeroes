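; Left-player paddle for the Pong mini-game in the Loading Screen System demo content, moving along the world X axis.
; Each Tick, collapsed graphs check X against the ±1500 limits and snap an out-of-range paddle back just inside.
; Otherwise it sets a new location from the MoveForward axis input, scaled by Speed and world delta seconds, keeping Y and Z unchanged.
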(event `self.ReceiveTick`
  (params (DeltaSeconds :type "Float (single-precision)"))
  (if (> (.x (`self.K2_GetActorLocation`)) 1500.0)
    (`self.K2_SetActorLocation` (`KismetMathLibrary.MakeVector` 1499.0 (.y (`self.K2_GetActorLocation`)) (.z (`self.K2_GetActorLocation`))))
    (elif (< (.x (`self.K2_GetActorLocation`)) -1500.0)
      (`self.K2_SetActorLocation` (`KismetMathLibrary.MakeVector` -1499.0 (.y (`self.K2_GetActorLocation`)) (.z (`self.K2_GetActorLocation`))))
      (else
        (`self.K2_SetActorLocation` (`KismetMathLibrary.MakeVector` (+ (* (`self.GetInputAxisValue`) (* (`GameplayStatics.GetWorldDeltaSeconds`) (`self.Speed`))) (.x (`self.K2_GetActorLocation`))) (.y (`self.K2_GetActorLocation`)) (.z (`self.K2_GetActorLocation`))))))))

(fn `UserConstructionScript`)