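; Showcase camera pawn that slides along world X through the loading screen system's demo content, with a spring-arm camera configured in the Construction Script.
; Configurable keys step a clamped signed speed multiplier right or left, zero it, or repossess LastPawn.
; Tick interpolates current speed toward the resulting target, eased or at a constant rate, and offsets the actor.
; Optional direction and stop sounds accompany speed changes, with movement volume following the multiplier.
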(event `Key|AnyKey` :consume false
  (params (Key :type "Key Structure"))
  ;[1 1 1] Input
  (:`Pressed`
    (bind _out_a (`self.is Key` Key (`self.Input Move Right`))
      (:`then`
        (`self.Move Right`))
      (:`else`
        (bind _out_a_2 (`self.is Key` _out_a (`self.Input Move Left`))
          (:`then`
            (`self.Move Left`))
          (:`else`
            (bind _out_a_3 (`self.is Key` _out_a_2 (`self.Input Stop Movement`))
              (:`then`
                (`self.Stop Movement`))
              (:`else`
                (`self.is Key` _out_a_3 (`self.Eject Pawn`)
                  (:`then`
                    (`self.Repossess Previous Pawn`)))))))))))

(event `Move Right`
  ;[1 1 1] Set Movement Speed
  (bind _result (`self.Change Speed With Sound`))
  (set `self.Target Speed` (* (`self.Speed`) _result)))

(event `Move Left`
  ;[1 1 1] Set Movement Speed
  (bind _result (`self.Change Speed With Sound` :!via `Decrease`))
  (set `self.Target Speed` (* (`self.Speed`) _result)))

(event `Stop Movement`
  ;[1 1 1] Set Movement Speed
  (`self.Change Speed With Sound` :!via `Zero`)
  (set `self.Target Speed` 0.0))

(event `self.ReceiveTick`
  (params (DeltaSeconds :type "Float (single-precision)"))
  ;[1 1 1] Update Movement
  (bind _returnvalue (`self.Accelerate` (`self.Current Speed`) (`self.Target Speed`) DeltaSeconds (`self.Acceleration`)))
  (bind _output_get (set `self.Current Speed` _returnvalue))
  (`self.K2_AddActorWorldOffset` (`KismetMathLibrary.MakeVector` (* _output_get (`GameplayStatics.GetWorldDeltaSeconds`)))))

(fn `Accelerate`
  (params (Current :type "Float (double-precision)") (Target :type "Float (double-precision)") (DeltaTime :type "Float (double-precision)") (InterpSpeed :type "Float (double-precision)"))
  (returns (ReturnValue :type "Float (double-precision)"))
  (return (select `bool` (`self.Use Constant Acceleration`) :`false` (`KismetMathLibrary.FInterpTo` Current Target DeltaTime InterpSpeed) :`true` (`KismetMathLibrary.FInterpTo_Constant` Current Target DeltaTime (select `bool` (`self.Use Constant Acceleration`) :`false` InterpSpeed :`true` (* InterpSpeed 20.0))))))

(fn `Decrease Speed Multiplier`
  (returns (Result :type "Float (double-precision)") (`Value Changed` :type Boolean))
  (bind _speed_multiplier (`self.Speed Multiplier`))
  (bind _speed_increments (`self.Speed Increments`))
  (bind _returnvalue (`KismetMathLibrary.FClamp` (+ _speed_multiplier -1.0) (* _speed_increments -1.0) _speed_increments))
  (bind _output_get (set `self.Speed Multiplier` _returnvalue))
  (return _output_get (!= _speed_multiplier _returnvalue)))

(fn `Increase Speed Multiplier`
  (returns (Result :type "Float (double-precision)") (`Value Changed` :type Boolean))
  (bind _speed_multiplier (`self.Speed Multiplier`))
  (bind _speed_increments (`self.Speed Increments`))
  (bind _returnvalue (`KismetMathLibrary.FClamp` (+ _speed_multiplier 1.0) (* _speed_increments -1.0) _speed_increments))
  (bind _output_get (set `self.Speed Multiplier` _returnvalue))
  (return _output_get (!= _speed_multiplier _returnvalue)))

(fn `Play Sound On Speed`
  (bind _moverightaudio (`self.MoveRightAudio`))
  (bind _moveleftaudio (`self.MoveLeftAudio`))
  (bind _speed_multiplier (`self.Speed Multiplier`))
  (`/Engine/EditorBlueprintResources/StandardMacros.CompareFloat` _speed_multiplier
    (:`>`
      (`AudioComponent.SetVolumeMultiplier` _moverightaudio (`self.Speed Multiplier`))
      (`AudioComponent.Play` _moverightaudio 0.0))
    (:`==`
      (`AudioComponent.Play` (`self.StopMovementAudio`) 0.0))
    (:`<`
      (`AudioComponent.SetVolumeMultiplier` _moveleftaudio (`KismetMathLibrary.Abs` _speed_multiplier))
      (`AudioComponent.Play` _moveleftaudio 0.0))))

(fn `Repossess Previous Pawn`
  (bind _lastpawn (`self.LastPawn`))
  (`/Engine/EditorBlueprintResources/StandardMacros.IsValid` _lastpawn
    (:`Is Valid`
      (`Controller.Possess` (`GameplayStatics.GetPlayerController` 0) _lastpawn))))

(fn `UserConstructionScript`
  (bind _springarm (`self.SpringArm`))
  (`SceneComponent.K2_SetRelativeRotation` (`self.Camera`) (`self.Camera Rotation`) false false)
  (`SceneComponent.K2_SetRelativeRotation` _springarm (`self.SpringArm Rotation`) false false)
  (set `SpringArmComponent.TargetArmLength` (`self.SpringArm Length`) _springarm))

(fn `Zero Speed Multiplier`
  (returns (Result :type "Float (double-precision)") (`Value Changed` :type Boolean))
  (locals (`Loc Value` :type "Float (double-precision)" :default 0.0))
  (bind _output_get (set `local.Loc Value` (`self.Speed Multiplier`)))
  (bind _output_get_2 (set `self.Speed Multiplier` 0.0))
  (return _output_get_2 (!= _output_get 0.0)))