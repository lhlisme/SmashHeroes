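; Base item pickup that flies to the player character and destroys itself when collected.
; After a short random delay on BeginPlay, it turns off physics on its Sphere, records its location and, if AutoMoveToPlayer is set, starts the MoveToPlayer timeline.
; Otherwise, the player's first overlap starts that timeline.
; The timeline lerps from the recorded location to the player's live position, then calls FinishCollectItem.
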(event `self.ReceiveBeginPlay`
  (`KismetSystemLibrary.Delay` (`KismetMathLibrary.RandomFloatInRange` 0.5 1.0))
  (`PrimitiveComponent.SetSimulatePhysics` (`self.Sphere`) false)
  (set `self.InitialActorLocation` (`self.K2_GetActorLocation`))
  (if (`self.AutoMoveToPlayer`)
    ;[1 1 1] Item朝玩家移动
    (bind (_direction _alpha) (`Timeline|MoveToPlayer` :!label _label)
      (:`Update`
        (`self.K2_SetActorLocation` (`KismetMathLibrary.VLerp` (`self.InitialActorLocation`) (`self.K2_GetActorLocation` (`/Game/BluePrints/Player/BP_PlayerController.PlayerCharacter` (`/Game/BluePrints/BP_SHFunctionLibrary.GetPlayerControllerBP`))) _alpha)))
      (:`Finished`
        (`self.FinishCollectItem`)))))

(event `self.ReceiveActorBeginOverlap`
  (params (OtherActor :type "Actor Object Reference"))
  (if (and (not (`self.AutoMoveToPlayer`)) (== OtherActor (`/Game/BluePrints/Player/BP_PlayerController.PlayerCharacter` (`/Game/BluePrints/BP_SHFunctionLibrary.GetPlayerControllerBP`))))
    (`/Engine/EditorBlueprintResources/StandardMacros.DoOnce` false
      (:`Completed`
        (goto _label)))))

(event `FinishCollectItem`
  (`self.K2_DestroyActor`))

(fn `UserConstructionScript`)