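; Game mode for Smash Heroes that sets up the player's character when play begins.
; On BeginPlay it caches every PlayerStart in the level, then calls CreatePlayer to add a local player with a controller.
; It spawns a CyberNinja character at a randomly chosen start, adjusting for collisions or skipping the spawn if still blocked, and has player controller 0 possess it.
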(event `self.ReceiveBeginPlay`
  (`self.GetPlayerStartPoints`)
  (`self.SpawnPlayer`))

(fn `GetPlayerStartPoints`
  (bind _outactors (`GameplayStatics.GetAllActorsOfClass` "/Script/Engine.PlayerStart"))
  (set `self.PlayerStartPoints` _outactors))

(fn `SpawnPlayer`
  (bind _playerstartpoints (`self.PlayerStartPoints`))
  (`GameplayStatics.CreatePlayer` -1)
  (bind _returnvalue (`|SpawnActorFromClass` "/Game/BluePrints/Player/BP_Character_CyberNinja.BP_Character_CyberNinja_C" (`self.GetTransform` (`|GetArrayItem` _playerstartpoints (`KismetMathLibrary.RandomIntegerInRange` 0 (- (`KismetArrayLibrary.Array_Length` _playerstartpoints) 1)))) "AdjustIfPossibleButDontSpawnIfColliding" "OverrideRootScale" null null))
  (`Controller.Possess` (`GameplayStatics.GetPlayerController` 0) _returnvalue))

(fn `UserConstructionScript`)