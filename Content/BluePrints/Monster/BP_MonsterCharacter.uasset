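; Monster character Blueprint that handles hit reactions, death and loot.
; While alive, damage plays a hit montage and red hit effect and updates hate toward the causer; health changes spawn a damage-text widget and trigger death handling once at zero life.
; On death it reports the kill to the game mode's MonsterManager, detaches its controller, changes collision to WorldDynamic and destroys itself after a delay, spawning loot once when destroyed.
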(event `self.OnHealthChanged`
  (params (DeltaValue :type "Float (single-precision)") (EventTags :type "GameplayTagContainer Structure (by ref)"))
  (`self.ShowDamageAmount` DeltaValue)
  (if (not (`self.IsAlive`))
    (`/Engine/EditorBlueprintResources/StandardMacros.DoOnce` false
      (:`Completed`
        (`self.HandleDead`)))))

(event `self.OnDamaged`
  (params (DamageAmount :type "Float (single-precision)") (HitInfo :type "HitResult Structure (by ref)") (DamageTags :type "GameplayTagContainer Structure (by ref)") (InstigatorCharacter :type "BaseCharacter Object Reference") (DamageCauser :type "Actor Object Reference"))
  ;[1 1 1] 受击时调用
  (if (`self.IsAlive`)
    (`self.PlayHitMontage` DamageCauser)
    (`self.UpdateHateValue` DamageAmount DamageCauser)
    (`self.PlayHitEffect` (struct :`R` 1.0 :`A` 1.0))))

(event `ShowDamageAmount`
  (params (Damage :type "Float (double-precision)"))
  (bind _returnvalue (`AddComponent|NODE_AddWC_DamageText-0` :`bManualAttachment` true :`RelativeTransform` (`self.GetTransform`)))
  (`/Game/BluePrints/Widgets/WC_DamageText.SetDamageText` _returnvalue Damage))

(event `self.OnDead`
  ;[1 1 1] 怪物死亡回调
  (`SHMonsterManager.IncreaseKilledMonsterCount` (`SHGameModeBase.MonsterManager` (`/Game/BluePrints/BP_SHFunctionLibrary.GetGameModeBP`)))
  (`self.DetachFromControllerPendingDestroy`)
  (`PrimitiveComponent.SetCollisionObjectType` (`self.CapsuleComponent`) "ECC_WorldDynamic")
  (`PrimitiveComponent.SetCollisionObjectType` (`self.Mesh`) "ECC_WorldDynamic")
  (`KismetSystemLibrary.PrintString` "MonsterDied")
  (`KismetSystemLibrary.Delay` 3.0)
  (`self.K2_DestroyActor`))

(event `self.ReceiveDestroyed`
  (`/Engine/EditorBlueprintResources/StandardMacros.DoOnce` false
    (:`Completed`
      (`self.SpawnLoot`))))

(fn `UserConstructionScript`)