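; Base gameplay ability for a character's ranged attack, firing projectiles that carry gameplay effects.
; On activation it notifies the behavior component, checks the character's RangeAttack, commits the ability, then plays its attack montage.
; Montage gameplay events build an effect container spec from the event tag and, if it has effects, spawn a projectile at each tag-matched spawn transform.
; Failed checks, montage blend-out, interruption or cancellation end the ability.
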(event `self.K2_ActivateAbility`
  (bind _asbase_character (cast `BaseCharacter` (`self.GetOwningActorFromActorInfo`))
    (:`then`
      (`BehaviorComponent.BeginRangeAttack` (`BaseCharacter.GetBehaviorComponent` _asbase_character))
      (bind _returnvalue (`BaseCharacter.RangeAttack` _asbase_character))
      (if _returnvalue
        (bind _returnvalue_2 (`self.K2_CommitAbility`))
        (if _returnvalue_2
          (bind (_asynctaskproxy _eventtag _eventdata) (`AbilityTask_PlayMontageWaitEvent.PlayMontageAndWaitForEvent` "None" (`BaseCharacter.GetAttackMontage` _asbase_character))
            (:`OnBlendOut`
              (`self.K2_EndAbility` :!label _label))
            (:`OnInterrupted`
              (goto _label))
            (:`OnCancelled`
              (goto _label))
            (:`EventReceived`
              (bind _returnvalue_3 (`self.MakeEffectContainerSpec` _eventtag _eventdata))
              (if (`SHBlueprintFunctionLibrary.DoesEffectContainerSpecHaveEffects` _returnvalue_3)
                (`self.SpawnProjectile` _returnvalue_3 _asbase_character _eventtag))))
          (else
            (goto _label)))
        (else
          (goto _label))))
    (:`CastFailed`
      (goto _label))))

(fn `SpawnProjectile`
  (params (EffectContainerSpec :type "SHGameplayEffectContainerSpec Structure") (Instigator :type "BaseCharacter Object Reference") (ProjectileTag :type "GameplayTag Structure"))
  (for _array_element (`BaseCharacter.GetProjectileSpawnTransforms` Instigator ProjectileTag)
    (`|SpawnActorFromClass` (`self.ProjectileClass`) _array_element "AlwaysSpawn" "OverrideRootScale" null EffectContainerSpec Instigator)))