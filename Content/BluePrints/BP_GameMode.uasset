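; Game mode that handles match start and game over, with Restart left as an empty event.
; StartGame gathers PlayerStart actors, creates a local player, spawns BP_Player_CyberNinja at a random start for player controller 0 to possess, then sets GameInProgress.
; GameOver plays a brief slow-motion beat, pauses the game, shows a reusable WB_GameFinish widget and switches to UI-only input.
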(event `self.ReceiveBeginPlay`)

(event `StartGame`
  (`self.GetPlayerStartPoints`)
  (`self.SpawnPlayer`)
  (if (not (`self.bGameInProgress`))
    (set `self.bGameInProgress` true)))

(event `GameOver`
  ;[1 1 1] 游戏结束时调用
  (`GameplayStatics.SetGlobalTimeDilation` 0.25)
  (`KismetSystemLibrary.Delay` 0.5)
  (`GameplayStatics.SetGlobalTimeDilation` 1.0)
  (`GameplayStatics.SetGamePaused` true)
  (`/Engine/EditorBlueprintResources/StandardMacros.IsValid` (`self.ResultUI`)
    (:`Is Valid`
      _)
    (:`Is Not Valid`
      (bind _returnvalue (`|CreateWidget` "/Game/BluePrints/Widgets/WB_GameFinish.WB_GameFinish_C"))
      (bind _output_get (set `self.ResultUI` _returnvalue))))
  (`UserWidget.AddToViewport` _output_get 0)
  (`WidgetBlueprintLibrary.SetInputMode_UIOnlyEx` (`/Game/BluePrints/BP_SHFunctionLibrary.GetPlayerControllerBP`) null "LockAlways"))

(event `Restart`)

(fn `GetPlayerStartPoints`
  (bind _outactors (`GameplayStatics.GetAllActorsOfClass` "/Script/Engine.PlayerStart"))
  (set `self.PlayerStartPoints` _outactors))

(fn `SpawnPlayer`
  (bind _playerstartpoints (`self.PlayerStartPoints`))
  (`GameplayStatics.CreatePlayer` -1)
  (bind _returnvalue (`|SpawnActorFromClass` "/Game/BluePrints/Player/BP_Player_CyberNinja.BP_Player_CyberNinja_C" (`self.GetTransform` (`|GetArrayItem` _playerstartpoints (`KismetMathLibrary.RandomIntegerInRange` 0 (- (`KismetArrayLibrary.Array_Length` _playerstartpoints) 1)))) "AdjustIfPossibleButDontSpawnIfColliding" "OverrideRootScale" null null))
  (`Controller.Possess` (`GameplayStatics.GetPlayerController` 0) _returnvalue))

(fn `UserConstructionScript`)