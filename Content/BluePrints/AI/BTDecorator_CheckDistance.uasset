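; Behavior Tree decorator that gates a branch by the distance between two actors stored in the Blackboard.
; It reads ActorA, ActorB and a Distance threshold from Blackboard keys, then compares the straight-line distance between the actors' locations to the threshold.
; An Operator variable selects the comparison, covering equality, inequality and ordered checks.
; The condition fails if either actor is invalid.
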(fn `PerformConditionCheck`
  (params (OwnerActor :type "Actor Object Reference"))
  (returns (ReturnValue :type Boolean))
  (bind _returnvalue (`BTFunctionLibrary.GetBlackboardValueAsActor` (`self.ActorA`)))
  (bind _returnvalue_2 (`BTFunctionLibrary.GetBlackboardValueAsActor` (`self.ActorB`)))
  (bind _returnvalue_3 (`BTFunctionLibrary.GetBlackboardValueAsFloat` (`self.Distance`)))
  (bind _returnvalue_4 (`KismetMathLibrary.VSize` (- (`Actor.K2_GetActorLocation` _returnvalue) (`Actor.K2_GetActorLocation` _returnvalue_2))))
  (if (and (`KismetSystemLibrary.IsValid` _returnvalue) (`KismetSystemLibrary.IsValid` _returnvalue_2))
    (return (select `/Game/BluePrints/Enums/EnumOperationType` (`self.Operator`) :`NewEnumerator0` (== _returnvalue_4 _returnvalue_3) :`NewEnumerator1` (!= _returnvalue_4 _returnvalue_3) :`NewEnumerator2` (< _returnvalue_4 _returnvalue_3) :`NewEnumerator3` (<= _returnvalue_4 _returnvalue_3) :`NewEnumerator4` (> _returnvalue_4 _returnvalue_3) :`NewEnumerator5` (>= _returnvalue_4 _returnvalue_3)))
    (else
      (return false))))