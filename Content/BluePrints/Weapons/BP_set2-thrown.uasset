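; Thrown weapon Blueprint from sci-fi set 2 that makes the look of its mesh customizable, with no active gameplay logic.
; The construction script creates a dynamic material instance for each of the first four material slots.
; Every instance receives the same tint, metallic, roughness and wear values from Blueprint variables.
; The second body metallic and roughness variables drive the blade parameters.
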(fn `UserConstructionScript`
  (for _array_element (`|MakeArray` 0 1 2 3)
    (bind _returnvalue (`PrimitiveComponent.CreateDynamicMaterialInstance` (`self.Mesh_scifi_set2_thrown`) _array_element null "None"))
    (`MaterialInstanceDynamic.SetVectorParameterValue` _returnvalue "ColorBase" (`self.Body Color Tint1`))
    (`MaterialInstanceDynamic.SetVectorParameterValue` _returnvalue "ColorGrip" (`self.Body Color Tint 2`))
    (`MaterialInstanceDynamic.SetScalarParameterValue` _returnvalue "Metallic Body" (`self.Body Metallic 1`))
    (`MaterialInstanceDynamic.SetScalarParameterValue` _returnvalue "Roughness Body" (`self.Body Roughness 1`))
    (`MaterialInstanceDynamic.SetScalarParameterValue` _returnvalue "Metallic Blade" (`self.Body Metallic 2`))
    (`MaterialInstanceDynamic.SetScalarParameterValue` _returnvalue "Roughness Blade" (`self.Body Roughness 2`))
    (`MaterialInstanceDynamic.SetScalarParameterValue` _returnvalue "Wear" (`self.Wear Amount`))
    (`MaterialInstanceDynamic.SetVectorParameterValue` _returnvalue "ColorMain" (`self.Blade Color`))))