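; BP_BasePortal is a portal actor that completes the mission when the player character enters it while it is enabled.
; EnablePortal makes the portal effect visible and sets the enabled flag.
; On overlap, it checks for the player character and that flag, then calls MissionCompleted on the game mode once through a DoOnce.
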(event `self.ReceiveActorBeginOverlap`
  (params (OtherActor :type "Actor Object Reference"))
  (if (and (== OtherActor (`/Game/BluePrints/BP_SHFunctionLibrary.GetPlayerCharacterBP`)) (`self.PortalEnabled`))
    (`/Engine/EditorBlueprintResources/StandardMacros.DoOnce` false
      (:`Completed`
        (`/Game/BluePrints/BP_GameMode.MissionCompleted` (`/Game/BluePrints/BP_SHFunctionLibrary.GetGameModeBP`))))))

(fn `EnablePortal`
  (`SceneComponent.SetVisibility` (`self.PortalEffect`) true false)
  (set `self.PortalEnabled` true))

(fn `UserConstructionScript`)