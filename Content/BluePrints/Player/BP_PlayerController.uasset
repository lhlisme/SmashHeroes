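; BP_PlayerController is the player's controller, managing the on-screen HUD and the crystal currency in the inventory.
; On first possession it caches the BP_PlayerCharacter and creates the mobile or PC HUD widget, once, toggling the virtual joystick with HUD visibility on mobile.
; AddCrystals and ConsumeCrystals wrap inventory calls on the crystal item, with adding also playing a purple emissive effect on the character.
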(event `self.ReceivePossess`
  (params (PossessedPawn :type "Pawn Object Reference"))
  ;[1 1 1] 初始化
  (`/Engine/EditorBlueprintResources/StandardMacros.DoOnce` false
    (:`Completed`
      (bind _asbp_player_character (cast `/Game/BluePrints/Player/BP_PlayerCharacter` PossessedPawn))
      (set `self.PlayerCharacter` _asbp_player_character)
      (`self.CreateHUD`))))

(event `CreateHUD`
  ;[1 1 1] 创建UI
  (`/Engine/EditorBlueprintResources/StandardMacros.IsValid` (`self.OnScreenControls`)
    (:`Is Valid`
      _)
    (:`Is Not Valid`
      (bind _returnvalue (`|CreateWidget` (select `bool` (`/Game/BluePrints/BP_SHFunctionLibrary.IsRunningOnMobile`) :`false` "/Game/BluePrints/Widgets/WB_HUD_PC.WB_HUD_PC_C" :`true` "/Game/BluePrints/Widgets/WB_HUD_Mobile.WB_HUD_Mobile_C" :!type "UserWidget Class Reference") self))
      (bind _output_get (set `self.OnScreenControls` _returnvalue))
      (`UserWidget.AddToViewport` _output_get 0)
      (message `/Game/BluePrints/Widgets/iHUD.UpdateIcons` (`self.OnScreenControls`))))
  (`self.ShowHUD` true))

(event `ShowHUD`
  (params (bIsVisible :type Boolean))
  (bind _onscreencontrols (`self.OnScreenControls`))
  ;[1 1 1] 显示或隐藏OnScreenControls(HUD)
  (`self.SetVirtualJoystickVisibility` (and bIsVisible (`/Game/BluePrints/BP_SHFunctionLibrary.IsRunningOnMobile`)))
  (`/Engine/EditorBlueprintResources/StandardMacros.IsValid` _onscreencontrols
    (:`Is Valid`
      (`Widget.SetVisibility` _onscreencontrols (select `bool` bIsVisible :`false` "Hidden" :`true` "SelfHitTestInvisible" :!type "ESlateVisibility Enum")))))

(fn `AddCrystals`
  (params (Amount :type Integer))
  (`self.AddInventoryItem` (`self.CrystalItem`) Amount)
  (`BaseCharacter.PlayEmissiveEffect` (`/Game/BluePrints/BP_SHFunctionLibrary.GetPlayerCharacterBP`) (struct :`R` 0.941177 :`G` 0.082353 :`B` 0.956863 :`A` 1.0)))

(fn `ConsumeCrystals`
  (params (Amount :type Integer))
  (returns (Success :type Boolean))
  (bind _returnvalue (`self.RemoveInventoryItem` (`self.CrystalItem`) Amount))
  (return _returnvalue))

(fn `UserConstructionScript`)