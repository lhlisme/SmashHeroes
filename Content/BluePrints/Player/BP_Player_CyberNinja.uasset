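; Player Blueprint for the CyberNinja character that maps combat input actions to character actions.
; Evade and Attack presses call TryEvade and TryAttack, while Guard press and release call HandleGuardStart and HandleGuardEnd, all defined outside this graph.
; Special activates GA_Base_Special directly by class through the Ability System, with a TODO for BeginSpecial.
; BeginPlay is disabled and the construction script only calls its parent.
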(event `InputAction|Evade`
  (params (Key :type "Key Structure"))
  (:`Pressed`
    (`self.TryEvade`)))

(event `InputAction|Guard`
  (params (Key :type "Key Structure"))
  (:`Pressed`
    (`self.HandleGuardStart`))
  (:`Released`
    (`self.HandleGuardEnd`)))

(event `InputAction|Special`
  (params (Key :type "Key Structure"))
  ;[1 1 1] TODO BeginSpecial
  (:`Pressed`
    (`AbilitySystemComponent.TryActivateAbilityByClass` (`self.AbilitySystem`) "/Game/BluePrints/Abilities/Base/GA_Base_Special.GA_Base_Special_C" true)))

(event `InputAction|Attack`
  (params (Key :type "Key Structure"))
  (:`Pressed`
    (`self.TryAttack`)))

(fn `UserConstructionScript`
  (`parent.UserConstructionScript`))