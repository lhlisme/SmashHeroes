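; Player character Blueprint for the Cyber Ninja, mapping combat input to Gameplay Ability System activations.
; Evade, Guard, Special and Attack each try to activate an ability by class; Attack uses the base melee ability.
; Evade, guard and combo state gate all but Special, and releasing Guard stops its montage and ends guarding.
; Left and right weapon attachment nodes in the Construction Script are disconnected and never run.
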(event `InputAction|Evade`
  (params (Key :type "Key Structure"))
  (:`Pressed`
    (if (and (not (`self.IsEvading`)) (not (`self.IsGuarding`)))
      (`AbilitySystemComponent.TryActivateAbilityByClass` (`self.AbilitySystem`) "/Game/BluePrints/Abilities/GA_CyberNinja_Evade.GA_CyberNinja_Evade_C" true))))

(event `InputAction|Guard`
  (params (Key :type "Key Structure"))
  (:`Pressed`
    (if (and (not (`self.IsEvading`)) (== (`self.ComboIndex`) 0))
      (`AbilitySystemComponent.TryActivateAbilityByClass` (`self.AbilitySystem`) "/Game/BluePrints/Abilities/GA_CyberNinja_Guard.GA_CyberNinja_Guard_C" true)))
  (:`Released`
    (if (`self.IsGuarding`)
      (`self.StopAnimMontage` "/Game/Animations/Montages/CyberNinja_Dual_Guard_Montage.CyberNinja_Dual_Guard_Montage")
      (`self.EndGuard`))))

(event `InputAction|Special`
  (params (Key :type "Key Structure"))
  (:`Pressed`
    (`AbilitySystemComponent.TryActivateAbilityByClass` (`self.AbilitySystem`) "/Game/BluePrints/Abilities/GA_CyberNinja_Special.GA_CyberNinja_Special_C" true)))

(event `InputAction|Attack`
  (params (Key :type "Key Structure"))
  (:`Pressed`
    (if (and (not (`self.IsEvading`)) (not (`self.IsGuarding`)))
      (`AbilitySystemComponent.TryActivateAbilityByClass` (`self.AbilitySystem`) "/Game/BluePrints/Abilities/GA_Base_MeleeAttack.GA_Base_MeleeAttack_C" true))))

(fn `UserConstructionScript`)